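; BP_Crystal is a collectible crystal that flies to the player and disappears when picked up.
; When the player pawn overlaps its collision sphere, it stores its location and plays a timeline.
; Each timeline update lerps the crystal toward the pawn's current location, so it homes in on a moving player, then the actor destroys itself when the timeline finishes.
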(event `self.Sphere_collision.OnComponentBeginOverlap`
  (params (OverlappedComponent :type "PrimitiveComponent Object Reference") (OtherActor :type "Actor Object Reference") (OtherComp :type "PrimitiveComponent Object Reference") (OtherBodyIndex :type Integer) (bFromSweep :type Boolean) (SweepResult :type "HitResult Structure (by ref)"))
  (if (== OtherActor (`GameplayStatics.GetPlayerPawn` 0))
    (set `self.LerpStartLocation` (`self.K2_GetActorLocation`))
    (bind (_direction _crystal_location) (`Timeline|TL_BlendAlpha`)
      (:`Update`
        (`self.K2_SetActorLocation` (`KismetMathLibrary.VLerp` (`self.LerpStartLocation`) (`self.K2_GetActorLocation` (`GameplayStatics.GetPlayerPawn` 0)) _crystal_location)))
      (:`Finished`
        (`self.K2_DestroyActor`)))))

(fn `UserConstructionScript`)