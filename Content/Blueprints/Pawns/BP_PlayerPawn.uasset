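; Player pawn for a rolling-ball game that restarts the level when it takes any damage.
; Forward/back and left/right axis inputs apply scaled torque to the Ball as an acceleration change, so it moves by physics rolling.
; The camera fades in on BeginPlay; on damage, RestartLevel starts a fade-out, waits briefly, then reopens the current level by name.
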(event `InputAxis|Move_forward/back`
  (params (AxisValue :type "Float (single-precision)"))
  (`self.NewFunction_0` AxisValue))

(event `self.ReceiveAnyDamage`
  (params (Damage :type "Float (single-precision)") (DamageType :type "DamageType Object Reference") (InstigatedBy :type "Controller Object Reference") (DamageCauser :type "Actor Object Reference"))
  (`self.RestartLevel`))

(event `InputAxis|Move_left/right`
  (params (AxisValue :type "Float (single-precision)"))
  (`self.NewFunction_1` AxisValue))

(event `self.ReceiveBeginPlay`
  (`PlayerCameraManager.StartCameraFade` :`self` (`GameplayStatics.GetPlayerCameraManager` 0) :`FromAlpha` 1.0 :`Duration` 2.0))

(fn `NewFunction_0`
  (params (A :type "Float (double-precision)"))
  (`PrimitiveComponent.AddTorqueInRadians` (`self.Ball`) (`KismetMathLibrary.MakeVector` 0.0 (* A (`self.Multiply`))) "None" true))

(fn `NewFunction_1`
  (params (A :type "Float (double-precision)"))
  (`PrimitiveComponent.AddTorqueInRadians` (`self.Ball`) (`KismetMathLibrary.MakeVector` (* A (`self.Multiply`))) "None" true))

(fn `UserConstructionScript`)