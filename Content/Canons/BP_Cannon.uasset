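; BP_Cannon is a cannon that automatically fires BP_Projectile actors on a repeating cycle from BeginPlay.
; Each cycle waits for the RatFire delay, then spawns a projectile at the SpawnPoint component's location and rotation.
; BarrelFireTimeline then animates the barrel's relative Y position, and its Finished output loops back to the delay, so the firing interval includes the animation length.
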(event `self.ReceiveBeginPlay`
  (`KismetSystemLibrary.Delay` (`self.RatFire`) :!label _label)
  (`self.SpawnProjectile`)
  (bind (_direction _barrellocationy) (`Timeline|BarrelFireTimeline` :!via `PlayFromStart`)
    (:`Update`
      (`self.ChangeBarrelYLocation` _barrellocationy))
    (:`Finished`
      (goto _label))))

(fn `ChangeBarrelYLocation`
  (params (NewLocation_Y :type "Float (double-precision)"))
  (`SceneComponent.K2_SetRelativeLocation` (`self.Cannon_Barrel`) (`KismetMathLibrary.MakeVector` 0.0 NewLocation_Y) false false))

(fn `SpawnProjectile`
  (`|SpawnActorFromClass` "/Game/Blueprints/Projectiles/BP_Projectile.BP_Projectile_C" (`KismetMathLibrary.MakeTransform` (`SceneComponent.GetSocketLocation` (`self.SpawnPoint`) "None") (`SceneComponent.K2_GetComponentRotation` (`self.SpawnPoint`))) "AlwaysSpawn" "OverrideRootScale" null null))

(fn `UserConstructionScript`)